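; PaperZD animation notify that applies the hit of a light attack.
; When received with a valid owning instance, it box-overlaps Pawns at the sequence render component's location, ignoring the owning actor.
; Each overlapped actor gets its name printed and takes a fixed amount of damage.
; Without a valid instance, it only draws a debug box of the HitBox extent.
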(event `self.OnReceiveNotify`
  (params (OwningInstance :type "PaperZDAnimInstance Object Reference"))
  (bind _returnvalue (`SceneComponent.K2_GetComponentLocation` (`self.SequenceRenderComponent`)))
  (`/Engine/EditorBlueprintResources/StandardMacros.IsValid` OwningInstance
    (:`Is Valid`
      (bind _outactors (`KismetSystemLibrary.BoxOverlapActors` _returnvalue (`self.HitBox`) (`|MakeArray` "ObjectTypeQuery3" :!type "EObjectTypeQuery Enum") null (`|MakeArray` (`PaperZDAnimInstance.GetOwningActor` OwningInstance))))
      (for _array_element _outactors
        (`KismetSystemLibrary.PrintString` (`KismetSystemLibrary.GetDisplayName` _array_element))
        (`GameplayStatics.ApplyDamage` _array_element 20.0)))
    (:`Is Not Valid`
      (`KismetSystemLibrary.DrawDebugBox` _returnvalue (`self.HitBox`)))))